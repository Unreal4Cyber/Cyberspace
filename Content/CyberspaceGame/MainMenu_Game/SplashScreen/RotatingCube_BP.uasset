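; Splash screen cube for the main menu, built as one cell of a 5x5 X/Z grid for a wave effect.
; ReturnSineSize maps XCoord and ZCoord to a hardcoded, roughly diagonal wave index times SineAngleOffset, with rows X=2 and X=3 identical.
; Three animation chains cover sine movement along Y, spin and uniform growth, but none is connected to an event, so the cube stays static.
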(event EventBeginPlay)

(event Collision|EventActorBeginOverlap
  (params (OtherActor :type Actor%20Object%20Reference)))

(event EventTick
  (params (DeltaSeconds :type Float%20%28single-precision%29)))

(fn ConstructionScript)

(fn ReturnSineSize
  (bind _zcoord (Variables|Default|GetzCoord))
  (bind _sineangleoffset (Variables|Default|GetsineAngleOffset))
  (switch int (Variables|Default|GetxCoord)
    (:0
      (switch int _zcoord
        (:0
          (bind _output_get (Variables|Default|SetvawePosition 4 :!label _label))
          (Variables|Default|SetsineAngleAbsolute (* _output_get _sineangleoffset)))
        (:1
          (bind _output_get_2 (Variables|Default|SetvawePosition 3 :!label _label_2))
          (Variables|Default|SetsineAngleAbsolute (* _output_get_2 _sineangleoffset)))
        (:2
          (bind _output_get_3 (Variables|Default|SetvawePosition 2 :!label _label_3))
          (Variables|Default|SetsineAngleAbsolute (* _output_get_3 _sineangleoffset)))
        (:3
          (bind _output_get_4 (Variables|Default|SetvawePosition 1))
          (Variables|Default|SetsineAngleAbsolute (* _output_get_4 _sineangleoffset)))
        (:4
          (bind _output_get_5 (Variables|Default|SetvawePosition 0 :!label _label_4))
          (Variables|Default|SetsineAngleAbsolute (* _output_get_5 _sineangleoffset)))))
    (:1
      (switch int _zcoord
        (:0
          (bind _output_get_6 (Variables|Default|SetvawePosition 5 :!label _label_5))
          (Variables|Default|SetsineAngleAbsolute (* _output_get_6 _sineangleoffset)))
        (:1
          (goto _label))
        (:2
          (goto _label_2))
        (:3
          (goto _label_3))
        (:4
          (goto _label_4))))
    (:2
      (switch int _zcoord
        (:0
          (bind _output_get_7 (Variables|Default|SetvawePosition 7 :!label _label_6))
          (Variables|Default|SetsineAngleAbsolute (* _output_get_7 _sineangleoffset)))
        (:1
          (bind _output_get_8 (Variables|Default|SetvawePosition 6 :!label _label_7))
          (Variables|Default|SetsineAngleAbsolute (* _output_get_8 _sineangleoffset)))
        (:2
          (goto _label_5))
        (:3
          (goto _label))
        (:4
          (goto _label_2))))
    (:3
      (switch int _zcoord
        (:0
          (goto _label_6))
        (:1
          (goto _label_7))
        (:2
          (goto _label_5))
        (:3
          (goto _label))
        (:4
          (goto _label_2))))
    (:4
      (switch int _zcoord
        (:0
          (bind _output_get_9 (Variables|Default|SetvawePosition 8))
          (Variables|Default|SetsineAngleAbsolute (* _output_get_9 _sineangleoffset)))
        (:1
          (goto _label_6))
        (:2
          (goto _label_7))
        (:3
          (goto _label_5))
        (:4
          (goto _label)))))
  (return (Variables|Default|GetsineAngleAbsolute)))