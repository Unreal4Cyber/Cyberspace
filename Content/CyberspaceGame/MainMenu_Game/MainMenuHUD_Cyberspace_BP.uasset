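; Main menu HUD for the Cyberspace game that sets up the menu screen and restores the player's saved audio settings.
; On BeginPlay it plays the menu music, locks the visible mouse in game-and-UI mode, positions the cursor and shows the MainMenu2 widget.
; LoadMainMenuSettings then copies volume and subtitle values from the MainMenuSettings save slot into the game instance, using its default values when no save exists.
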(event EventBeginPlay
  (bind _returnvalue (Game|GetPlayerController 0))
  (Audio|PlaySound2D "/Game/CyberspaceGame/MainMenu_Game/Sounds/1950467_tension-action-loop_by_symphony-of-specter.1950467_tension-action-loop_by_symphony-of-specter")
  (Input|SetInputModeGameandUI _returnvalue 0 "LockAlways" true)
  (bind _returnvalue_2 (UserInterface|CreateWidget "/Game/CyberspaceGame/MainMenu_Game/MainMenu2.MainMenu2_C"))
  (UserInterface|Viewport|AddtoViewport _returnvalue_2 0)
  (Variables|/Script/Engine.PlayerController|SetbShowMouseCursor _returnvalue true)
  (Class|PlayerController|SetMouseLocation _returnvalue 340 470)
  (CallFunction|LoadMainMenuSettings))

(fn ConstructionScript)

(fn LoadMainMenuSettings
  (bind _returnvalue (SaveGame|DoesSaveGameExist "MainMenuSettings"))
  (if _returnvalue
    ;[0.6953 1 0.6342] Load Main Menu Settings from disk (Saved settings exist)
    (bind _returnvalue_2 (SaveGame|LoadGamefromSlot "MainMenuSettings"))
    (bind _assave_main_menu_settings (Utilities|Casting|CastToSaveMainMenuSettings _returnvalue_2))
    (bind _asmain_menu_game_instance (Utilities|Casting|CastToMainMenuGameInstance (Game|GetGameInstance)))
    (Variables|/Game/CyberspaceGame/MainMenu_Game/MainMenuGameInstance.MainMenuGameInstance_C|SetaudioSettMasterVolume _asmain_menu_game_instance (Variables|/Game/CyberspaceGame/MainMenu_Game/SaveMainMenuSettings.SaveMainMenuSettings_C|GetaudioSettMasterVolumeSaved _assave_main_menu_settings))
    (Variables|/Game/CyberspaceGame/MainMenu_Game/MainMenuGameInstance.MainMenuGameInstance_C|SetaudioSettMusicVolume _asmain_menu_game_instance (Variables|/Game/CyberspaceGame/MainMenu_Game/SaveMainMenuSettings.SaveMainMenuSettings_C|GetaudioSettMusicVolumeSaved _assave_main_menu_settings))
    (Variables|/Game/CyberspaceGame/MainMenu_Game/MainMenuGameInstance.MainMenuGameInstance_C|SetaudioSettSpeechVolume _asmain_menu_game_instance (Variables|/Game/CyberspaceGame/MainMenu_Game/SaveMainMenuSettings.SaveMainMenuSettings_C|GetaudioSettSpeechVolumeSaved _assave_main_menu_settings))
    (Variables|/Game/CyberspaceGame/MainMenu_Game/MainMenuGameInstance.MainMenuGameInstance_C|SetaudioSettVideoVolume _asmain_menu_game_instance (Variables|/Game/CyberspaceGame/MainMenu_Game/SaveMainMenuSettings.SaveMainMenuSettings_C|GetaudioSettVideoVolumeSaved _assave_main_menu_settings))
    (Variables|/Game/CyberspaceGame/MainMenu_Game/MainMenuGameInstance.MainMenuGameInstance_C|SetaudioSettSubtitles _asmain_menu_game_instance (Variables|/Game/CyberspaceGame/MainMenu_Game/SaveMainMenuSettings.SaveMainMenuSettings_C|GetaudioSettSubtitlesSaved _assave_main_menu_settings))
    (else
      ;[1 1 1] Put default values to global variables (Saved settings do not exist)
      (bind _asmain_menu_game_instance_2 (Utilities|Casting|CastToMainMenuGameInstance (Game|GetGameInstance)))
      (Variables|/Game/CyberspaceGame/MainMenu_Game/MainMenuGameInstance.MainMenuGameInstance_C|SetaudioSettMasterVolume _asmain_menu_game_instance_2 (Variables|/Game/CyberspaceGame/MainMenu_Game/MainMenuGameInstance.MainMenuGameInstance_C|GetaudioSettMasterVolumeDefaultValue _asmain_menu_game_instance_2))
      (Variables|/Game/CyberspaceGame/MainMenu_Game/MainMenuGameInstance.MainMenuGameInstance_C|SetaudioSettMusicVolume _asmain_menu_game_instance_2 (Variables|/Game/CyberspaceGame/MainMenu_Game/MainMenuGameInstance.MainMenuGameInstance_C|GetaudioSettMusicVolumeDefaultValue _asmain_menu_game_instance_2))
      (Variables|/Game/CyberspaceGame/MainMenu_Game/MainMenuGameInstance.MainMenuGameInstance_C|SetaudioSettSpeechVolume _asmain_menu_game_instance_2 (Variables|/Game/CyberspaceGame/MainMenu_Game/MainMenuGameInstance.MainMenuGameInstance_C|GetaudioSettSpeechVolumeDefaultValue _asmain_menu_game_instance_2))
      (Variables|/Game/CyberspaceGame/MainMenu_Game/MainMenuGameInstance.MainMenuGameInstance_C|SetaudioSettVideoVolume _asmain_menu_game_instance_2 (Variables|/Game/CyberspaceGame/MainMenu_Game/MainMenuGameInstance.MainMenuGameInstance_C|GetaudioSettVideoVolumeDefaultValue _asmain_menu_game_instance_2))
      (Variables|/Game/CyberspaceGame/MainMenu_Game/MainMenuGameInstance.MainMenuGameInstance_C|SetaudioSettSubtitles _asmain_menu_game_instance_2 (Variables|/Game/CyberspaceGame/MainMenu_Game/MainMenuGameInstance.MainMenuGameInstance_C|GetaudioSettSubtitlesDefaultValue _asmain_menu_game_instance_2))))
  (return))